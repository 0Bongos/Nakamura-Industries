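; Pressure-base actor that switches two referenced laser gates on while its Box is overlapped and off when the overlap ends.
; Overlap events toggle the gates' collision and visibility and set the base material's Active parameter to light it up.
; Positional audio events play switch sounds and looping hums, with HumOn and PowerOn flags guarding repeats; Lazer_grid_off plays on both activation and deactivation.
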(event `self.Box.OnComponentBeginOverlap`
  (params (OverlappedComponent :type "PrimitiveComponent Object Reference") (OtherActor :type "Actor Object Reference") (OtherComp :type "PrimitiveComponent Object Reference") (OtherBodyIndex :type Integer) (bFromSweep :type Boolean) (SweepResult :type "HitResult Structure (by ref)"))
  (bind _lasergatetwo (`self.Lasergatetwo`))
  (bind _lasergatereference (`self.LaserGateReference`))
  (bind _box (`self.Box`))
  (bind _power_on (`self.Power on`))
  (bind _returnvalue (`self.K2_GetActorLocation` _lasergatetwo))
  (bind _returnvalue_2 (`self.K2_GetActorLocation` _lasergatereference))
  (`FMODBlueprintStatics.PlayEventAtLocation` "/Game/FMOD/Events/Cube_Base_on.Cube_Base_on" (`KismetMathLibrary.Conv_VectorToTransform` (`SceneComponent.K2_GetComponentLocation` _box)))
  (if (not (`self.HumOn`))
    (bind _returnvalue_3 (`FMODBlueprintStatics.PlayEventAtLocation` "/Game/FMOD/Events/Light_Hum_1.Light_Hum_1" (`KismetMathLibrary.Conv_VectorToTransform` (`SceneComponent.K2_GetComponentLocation` _box))))
    (set `self.HumOn` true)
    (`PrimitiveComponent.CreateDynamicMaterialInstance` (`self.Base`) 0 "/Game/Material/CubeMatss/CubeBase/Clean/CleanCubeBase-Mat_Inst.CleanCubeBase-Mat_Inst" "None")
    (`MeshComponent.SetScalarParameterValueOnMaterials` (`self.Base`) "Active" 120.0)
    (`self.SetActorEnableCollision` _lasergatereference true)
    (`self.SetActorHiddenInGame` _lasergatereference false)
    (`self.SetActorEnableCollision` _lasergatetwo true)
    (`self.SetActorHiddenInGame` _lasergatetwo false)
    (if (not (`self.Power on`))
      (`FMODBlueprintStatics.PlayEventAtLocation` "/Game/FMOD/Events/Lazer_grid_off.Lazer_grid_off" (`KismetMathLibrary.Conv_VectorToTransform` _returnvalue))
      (`FMODBlueprintStatics.PlayEventAtLocation` "/Game/FMOD/Events/Lazer_grid_off.Lazer_grid_off" (`KismetMathLibrary.Conv_VectorToTransform` _returnvalue_2))
      (if (not _power_on)
        (bind _returnvalue_4 (`FMODBlueprintStatics.PlayEventAtLocation` "/Game/FMOD/Events/Lazer_Hum.Lazer_Hum" (`KismetMathLibrary.Conv_VectorToTransform` _returnvalue)))
        (if (not _power_on)
          (bind _returnvalue_5 (`FMODBlueprintStatics.PlayEventAtLocation` "/Game/FMOD/Events/Lazer_Hum.Lazer_Hum" (`KismetMathLibrary.Conv_VectorToTransform` _returnvalue_2)))
          (set `self.Power on` true))))))

(event `self.Box.OnComponentEndOverlap`
  (params (OverlappedComponent :type "PrimitiveComponent Object Reference") (OtherActor :type "Actor Object Reference") (OtherComp :type "PrimitiveComponent Object Reference") (OtherBodyIndex :type Integer))
  (bind _lasergatetwo (`self.Lasergatetwo`))
  (bind _lasergatereference (`self.LaserGateReference`))
  (`FMODBlueprintStatics.EventInstanceStop` (stale `self.Box.OnComponentBeginOverlap` _returnvalue_3))
  (set `self.HumOn` false)
  (`FMODBlueprintStatics.PlayEventAtLocation` "/Game/FMOD/Events/Cube_Base_off.Cube_Base_off" (`KismetMathLibrary.Conv_VectorToTransform` (`SceneComponent.K2_GetComponentLocation` (`self.Box`))))
  (`PrimitiveComponent.CreateDynamicMaterialInstance` (`self.Base`) 0 "/Game/Material/CubeMatss/CubeBase/Clean/CleanCubeBase-Mat_Inst.CleanCubeBase-Mat_Inst" "None")
  (`MeshComponent.SetScalarParameterValueOnMaterials` (`self.Base`) "Active" 0.0)
  (`self.SetActorEnableCollision` _lasergatereference false)
  (`self.SetActorHiddenInGame` _lasergatereference true)
  (`self.SetActorEnableCollision` _lasergatetwo false)
  (`self.SetActorHiddenInGame` _lasergatetwo true)
  (`FMODBlueprintStatics.EventInstanceStop` (stale `self.Box.OnComponentBeginOverlap` _returnvalue_4))
  (`FMODBlueprintStatics.EventInstanceStop` (stale `self.Box.OnComponentBeginOverlap` _returnvalue_5))
  (if (`self.Power on`)
    (`FMODBlueprintStatics.PlayEventAtLocation` "/Game/FMOD/Events/Lazer_grid_off.Lazer_grid_off" (`KismetMathLibrary.Conv_VectorToTransform` (`self.K2_GetActorLocation` _lasergatereference)))
    (`FMODBlueprintStatics.PlayEventAtLocation` "/Game/FMOD/Events/Lazer_grid_off.Lazer_grid_off" (`KismetMathLibrary.Conv_VectorToTransform` (`self.K2_GetActorLocation` _lasergatetwo)))
    (set `self.Power on` false)))

(fn `UserConstructionScript`)