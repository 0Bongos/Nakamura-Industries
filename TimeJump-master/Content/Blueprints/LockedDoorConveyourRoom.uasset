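; Locked door for the conveyor room that opens when the referenced key actor overlaps its Box trigger.
; The correct key destroys the box platform, turns the point light and two DoorLight actors green, then plays a timeline.
; Timeline updates set both doors to hardcoded world positions, with the track output unused, and set StartPoop on the referenced BoxPooper_3Colour.
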(event `self.Box.OnComponentBeginOverlap`
  (params (OverlappedComponent :type "PrimitiveComponent Object Reference") (OtherActor :type "Actor Object Reference") (OtherComp :type "PrimitiveComponent Object Reference") (OtherBodyIndex :type Integer) (bFromSweep :type Boolean) (SweepResult :type "HitResult Structure (by ref)"))
  (set `self.CorrectKey` (== OtherActor (`self.KeyReference`)))
  (if (`self.CorrectKey`)
    (`self.K2_DestroyActor` (`self.BoxPlatform`))
    (`LightComponent.SetLightColor` (`self.PointLight`) (struct :`R` 0.119792 :`G` 0.958333 :`B` 0.171363 :`A` 1.0) true)
    (bind _asdoor_light (cast `/Game/Blueprints/DoorLight` (`self.PoopBoxLight`)))
    (`LightComponent.SetLightColor` (`Light.LightComponent` _asdoor_light) (struct :`R` 0.065592 :`G` 0.96875 :`B` 0.307653 :`A` 1.0) true)
    (bind _asdoor_light_2 (cast `/Game/Blueprints/DoorLight` (`self.Door Light`)))
    (`LightComponent.SetLightColor` (`Light.LightComponent` _asdoor_light_2) (struct :`R` 0.065592 :`G` 0.96875 :`B` 0.307653 :`A` 1.0) true)
    (bind (_direction _newtrack_0) (`Timeline|Timeline_1`)
      (:`Update`
        (`SceneComponent.K2_SetWorldLocation` (`Actor.RootComponent` (`self.DoorRight`)) (3435.217529 6477.983887 2549.0) false false)
        (`SceneComponent.K2_SetWorldLocation` (`Actor.RootComponent` (`self.DoorLeft`)) (`KismetMathLibrary.MakeVector` 1385.0 (+ (* 0.0 (`self.NegativeDistance`)) 7845.0) 2195.0) false false)
        (bind _asbox_pooper_3colour (cast `/Game/Blueprints/BoxPooper_3Colour` (`self.BoxPooperRef`)))
        (set `/Game/Blueprints/BoxPooper_3Colour.StartPoop` true _asbox_pooper_3colour)))))

(fn `UserConstructionScript`)