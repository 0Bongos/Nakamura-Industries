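; LockedDoor is an actor that slides a pair of doors open when a specific key actor enters its trigger box.
; The Box overlap event compares the incoming actor with KeyReference and, on a match, plays a timeline.
; Each update moves the referenced DoorRight and DoorLeft actors along world X by the track value times NegativeDistance and OpenDistance respectively, from hardcoded world positions.
; No logic closes the doors again.
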(event `self.Box.OnComponentBeginOverlap`
  (params (OverlappedComponent :type "PrimitiveComponent Object Reference") (OtherActor :type "Actor Object Reference") (OtherComp :type "PrimitiveComponent Object Reference") (OtherBodyIndex :type Integer) (bFromSweep :type Boolean) (SweepResult :type "HitResult Structure (by ref)"))
  (set `self.CorrectKey` (== OtherActor (`self.KeyReference`)))
  (if (`self.CorrectKey`)
    (bind (_direction _newtrack_0) (`Timeline|Timeline_1`)
      (:`Update`
        (`SceneComponent.K2_SetWorldLocation` (`Actor.RootComponent` (`self.DoorRight`)) (`KismetMathLibrary.MakeVector` (- (* _newtrack_0 (`self.NegativeDistance`)) 3654.899902) 6429.999023 145.0) false false)
        (`SceneComponent.K2_SetWorldLocation` (`Actor.RootComponent` (`self.DoorLeft`)) (`KismetMathLibrary.MakeVector` (- (* _newtrack_0 (`self.OpenDistance`)) 3529.998535) 6429.998535 145.0) false false)))))

(fn `UserConstructionScript`)