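; Level 2 keypad that accepts a specific key actor and grants third-floor lift access.
; When the referenced key overlaps its box, the character drops it, the unlock sound plays once and the key is destroyed.
; It then fires particles, swaps the panel to the unlocked material, turns the light cyan and sets the third-floor access flag on the referenced lift blueprint.
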(event `self.Box.OnComponentBeginOverlap`
  (params (OverlappedComponent :type "PrimitiveComponent Object Reference") (OtherActor :type "Actor Object Reference") (OtherComp :type "PrimitiveComponent Object Reference") (OtherBodyIndex :type Integer) (bFromSweep :type Boolean) (SweepResult :type "HitResult Structure (by ref)"))
  (bind _keyreference (`self.KeyReference`))
  (set `self.CorrectKey` (== OtherActor _keyreference))
  (if (`self.CorrectKey`)
    (`/Game/FirstPersonBP/Blueprints/FirstPersonCharacter.Drop` (`self.Character`))
    (if (not (`self.DoorUnlocked`))
      (`FMODBlueprintStatics.PlayEventAtLocation` "/Game/FMOD/Events/Keypad_Unlock.Keypad_Unlock" (`KismetMathLibrary.Conv_VectorToTransform` (`SceneComponent.K2_GetComponentLocation` (`self.KeyPanel`))))
      (set `self.DoorUnlocked` true))
    (`self.K2_DestroyActor` _keyreference)
    (`ActorComponent.Activate` (`self.ParticleSystem`) false)
    (`KismetSystemLibrary.Delay` 0.2)
    (`ActorComponent.Activate` (`self.ParticleSystem`) false)
    (`PrimitiveComponent.SetMaterial` (`self.KeyPanel`) 0 "/Game/Material/CardReaderMats/Unlocked/Unlocked.Unlocked")
    (`LightComponent.SetLightColor` (`self.PointLight`) (struct :`G` 0.958333 :`B` 0.958333 :`A` 1.0) true)
    (bind _aslift_blueprint (cast `/Game/Blueprints/Lift_blueprint` (`self.LiftReference`)))
    (set `/Game/Blueprints/Lift_blueprint.3rdflooracess` true _aslift_blueprint)))

(fn `UserConstructionScript`)