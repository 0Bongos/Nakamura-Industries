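; Key-locked door panel that opens when one specific referenced key actor overlaps its Box trigger.
; The key is destroyed and particles activate, then after a short delay a one-time unlock plays audio, swaps the panel material and recolors both lights.
; A timeline then drives the right door from hard-coded world coordinates, but the DoorInMotion guard lets the open sound and move run only on its first update.
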(event `self.Box.OnComponentBeginOverlap`
  (params (OverlappedComponent :type "PrimitiveComponent Object Reference") (OtherActor :type "Actor Object Reference") (OtherComp :type "PrimitiveComponent Object Reference") (OtherBodyIndex :type Integer) (bFromSweep :type Boolean) (SweepResult :type "HitResult Structure (by ref)"))
  (bind _keypanel (`self.KeyPanel`))
  (bind _keyreference (`self.KeyReference`))
  (set `self.CorrectKey` (== OtherActor _keyreference))
  (if (`self.CorrectKey`)
    (`self.K2_DestroyActor` _keyreference)
    (`ActorComponent.Activate` (`self.ParticleSystem`) false)
    (`KismetSystemLibrary.Delay` 0.2)
    (`ActorComponent.Activate` (`self.ParticleSystem`) false)
    (if (not (`self.DoorUnlocked`))
      (`FMODBlueprintStatics.PlayEventAtLocation` "/Game/FMOD/Events/Keypad_Unlock.Keypad_Unlock" (`KismetMathLibrary.Conv_VectorToTransform` (`SceneComponent.K2_GetComponentLocation` (`self.KeyPanel`))))
      (set `self.DoorUnlocked` true)
      (`PrimitiveComponent.SetMaterial` _keypanel 0 "/Game/Material/CardReaderMats/Unlocked/Unlocked.Unlocked")
      (`LightComponent.SetLightColor` (`self.PointLight`) (struct :`G` 0.846507 :`B` 0.958333 :`A` 1.0) true)
      (bind _asdoor_light (cast `/Game/Blueprints/DoorLight` (`self.DoorLight`)))
      (`LightComponent.SetLightColor` (`Light.LightComponent` _asdoor_light) (struct :`G` 0.94306 :`B` 0.96875 :`A` 1.0) true)
      (bind (_direction _newtrack_0) (`Timeline|Timeline_1`)
        (:`Update`
          (if (not (`self.DoorInMotion`))
            (`FMODBlueprintStatics.PlayEventAtLocation` "/Game/FMOD/Events/Door_Open.Door_Open" (`KismetMathLibrary.Conv_VectorToTransform` (`SceneComponent.K2_GetComponentLocation` _keypanel)))
            (set `self.DoorInMotion` true)
            (`SceneComponent.K2_SetWorldLocation` (`Actor.RootComponent` (`self.DoorRight`)) (`KismetMathLibrary.MakeVector` (+ (* _newtrack_0 (`self.NegativeDistance`)) 2576.0) 10001.0 2419.0) false false)))))))

(fn `UserConstructionScript`)