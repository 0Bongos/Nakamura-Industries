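; A keypad-locked door that opens when a specific key actor enters its trigger box.
; A matching overlap destroys the key, fires particles, then after a short delay unlocks once, swapping the panel material, recoloring the light and playing an unlock sound.
; A timeline then moves the separate DoorRight actor along Z from hardcoded world coordinates, with a flag limiting the opening sound to one play.
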(event `self.Box.OnComponentBeginOverlap`
  (params (OverlappedComponent :type "PrimitiveComponent Object Reference") (OtherActor :type "Actor Object Reference") (OtherComp :type "PrimitiveComponent Object Reference") (OtherBodyIndex :type Integer) (bFromSweep :type Boolean) (SweepResult :type "HitResult Structure (by ref)"))
  (bind _keyreference (`self.KeyReference`))
  (set `self.CorrectKey` (== OtherActor _keyreference))
  (if (`self.CorrectKey`)
    (`self.K2_DestroyActor` _keyreference)
    (`ActorComponent.Activate` (`self.ParticleSystem`) false)
    (`KismetSystemLibrary.Delay` 0.2)
    (`ActorComponent.Activate` (`self.ParticleSystem`) false)
    (if (not (`self.DoorUnlocked`))
      (`FMODBlueprintStatics.PlayEventAtLocation` "/Game/FMOD/Events/Keypad_Unlock.Keypad_Unlock" (`KismetMathLibrary.Conv_VectorToTransform` (`SceneComponent.K2_GetComponentLocation` (`self.KeyPanel`))))
      (set `self.DoorUnlocked` true)
      (`PrimitiveComponent.SetMaterial` (`self.KeyPanel`) 0 "/Game/Material/CardReaderMats/Unlocked/Unlocked.Unlocked")
      (`LightComponent.SetLightColor` (`self.PointLight`) (struct :`R` 0.026519 :`G` 0.958333 :`B` 0.881978 :`A` 1.0) true)
      (bind (_direction _newtrack_0) (`Timeline|Timeline_1`)
        (:`Update`
          (if (not (`self.DoorInMotion`))
            (`FMODBlueprintStatics.PlayEventAtLocation` "/Game/FMOD/Events/Door_Open.Door_Open" (`KismetMathLibrary.Conv_VectorToTransform` (`SceneComponent.K2_GetComponentLocation` (`Actor.RootComponent` (`self.DoorRight`)))))
            (set `self.DoorInMotion` true))
          (`SceneComponent.K2_SetWorldLocation` (`Actor.RootComponent` (`self.DoorRight`)) (`KismetMathLibrary.MakeVector` 1355.0 8028.0 (+ (* _newtrack_0 (`self.OpenDistance`)) 2055.0)) false false))))))

(fn `UserConstructionScript`)