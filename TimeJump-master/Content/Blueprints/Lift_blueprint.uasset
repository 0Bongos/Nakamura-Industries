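; Elevator that carries the first-person character from ground, first or second floor up to the highest floor its access flags allow.
; Floor triggers record the player's floor and recall the lift from higher floors by reversing the matching timeline.
; Entering the lift's box picks a destination, updates lift-position booleans and plays one timeline per floor pair, setting hardcoded world locations.
; Access flags are only read here; three older relative-location timelines are unused.
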(event `self.Box.OnComponentBeginOverlap`
  (params (OverlappedComponent :type "PrimitiveComponent Object Reference") (OtherActor :type "Actor Object Reference") (OtherComp :type "PrimitiveComponent Object Reference") (OtherBodyIndex :type Integer) (bFromSweep :type Boolean) (SweepResult :type "HitResult Structure (by ref)"))
  (cast `/Game/FirstPersonBP/Blueprints/FirstPersonCharacter` OtherActor)
  (if (`self.player2nd floor`)
    (if (`self.3rdflooracess`)
      (set `self.Ele1st` false)
      (set `self.Ele2nd` false)
      (set `self.Ele3rdWin` true)
      (bind (_direction _newtrack_0) (`Timeline|Timeline_6` :!label _label)
        (:`Update`
          (`SceneComponent.K2_SetWorldLocation` (`self.Lift`) (`KismetMathLibrary.MakeVector` 2145.0 8000.0 (+ (* _newtrack_0 (`self.+1`)) 2765.0)) false false)))
      (else
        (set `self.Ele1st` false)
        (set `self.Ele2nd` true)
        (set `self.Ele3rdWin` false)
        (set `self.PlayerGround` false)
        (set `self.Player1stfloor` false)
        (set `self.player2nd floor` true)))
    (elif (`self.Player1stfloor`)
      (if (`self.3rdflooracess`)
        (set `self.Ele1st` false)
        (set `self.Ele2nd` false)
        (set `self.Ele3rdWin` true)
        (bind (_direction_2 _newtrack_0_2) (`Timeline|Timeline_7` :!label _label_2)
          (:`Update`
            (`SceneComponent.K2_SetWorldLocation` (`self.Lift`) (`KismetMathLibrary.MakeVector` 2145.0 8000.0 (+ (* _newtrack_0_2 (`self.+2`)) 2415.0)) false false)))
        (elif (`self.2ndFlooraces`)
          (set `self.Ele1st` false)
          (set `self.Ele2nd` true)
          (set `self.Ele3rdWin` false)
          (set `self.PlayerGround` false)
          (set `self.Player1stfloor` false)
          (set `self.player2nd floor` true)
          (bind (_direction_3 _newtrack_0_3) (`Timeline|Timeline_9` :!label _label_3)
            (:`Update`
              (`SceneComponent.K2_SetWorldLocation` (`self.Lift`) (`KismetMathLibrary.MakeVector` 2145.0 8000.0 (+ (* _newtrack_0_3 (`self.+1`)) 2415.0)) false false)))
          (else
            (set `self.Ele1st` true)
            (set `self.Ele2nd` false)
            (set `self.Ele3rdWin` false)
            (set `self.PlayerGround` false)
            (set `self.Player1stfloor` true)
            (set `self.player2nd floor` false))))
      (elif (`self.PlayerGround`)
        (if (`self.3rdflooracess`)
          (set `self.Ele1st` false)
          (set `self.Ele2nd` false)
          (set `self.Ele3rdWin` true)
          (bind (_direction_4 _newtrack_0_4) (`Timeline|Timeline_8` :!label _label_4)
            (:`Update`
              (`SceneComponent.K2_SetWorldLocation` (`self.Lift`) (`KismetMathLibrary.MakeVector` 2145.0 8000.0 (+ (* _newtrack_0_4 (`self.+3`)) 2065.0)) false false)))
          (elif (`self.2ndFlooraces`)
            (set `self.Ele1st` false)
            (set `self.Ele2nd` true)
            (set `self.Ele3rdWin` false)
            (set `self.PlayerGround` false)
            (set `self.Player1stfloor` false)
            (set `self.player2nd floor` true)
            (bind (_direction_5 _newtrack_0_5) (`Timeline|Timeline_10` :!label _label_5)
              (:`Update`
                (`SceneComponent.K2_SetWorldLocation` (`self.Lift`) (`KismetMathLibrary.MakeVector` 2145.0 8000.0 (+ (* _newtrack_0_5 (`self.+2`)) 2065.0)) false false)))
            (else
              (set `self.Ele1st` true)
              (set `self.Ele2nd` false)
              (set `self.Ele3rdWin` false)
              (set `self.PlayerGround` false)
              (set `self.Player1stfloor` true)
              (set `self.player2nd floor` false)
              (bind (_direction_6 _newtrack_0_6) (`Timeline|Timeline_11` :!label _label_6)
                (:`Update`
                  (`SceneComponent.K2_SetWorldLocation` (`self.Lift`) (`KismetMathLibrary.MakeVector` 2145.0 8000.0 (+ (* _newtrack_0_6 (`self.+1`)) 2065.0)) false false))))))))))

(event `self.Ground.OnComponentBeginOverlap`
  (params (OverlappedComponent :type "PrimitiveComponent Object Reference") (OtherActor :type "Actor Object Reference") (OtherComp :type "PrimitiveComponent Object Reference") (OtherBodyIndex :type Integer) (bFromSweep :type Boolean) (SweepResult :type "HitResult Structure (by ref)"))
  (set `self.PlayerGround` true)
  (set `self.Player1stfloor` false)
  (set `self.player2nd floor` false)
  (if (`self.Ele3rdWin`) :!label _label_7
    (if (`self.player2nd floor`)
      (set `self.Ele1st` false)
      (set `self.Ele2nd` true)
      (set `self.Ele3rdWin` false)
      (goto _label :!via `Reverse`)
      (elif (`self.Player1stfloor`)
        (set `self.Ele1st` true)
        (set `self.Ele2nd` false)
        (set `self.Ele3rdWin` false)
        (goto _label_2 :!via `Reverse`)
        (elif (`self.PlayerGround`)
          (set `self.Ele1st` false)
          (set `self.Ele2nd` false)
          (set `self.Ele3rdWin` false)
          (goto _label_4 :!via `Reverse`))))
    (elif (`self.Ele2nd`)
      (if (`self.Player1stfloor`)
        (set `self.Ele1st` true)
        (set `self.Ele2nd` false)
        (set `self.Ele3rdWin` false)
        (goto _label_3 :!via `Reverse`)
        (elif (`self.PlayerGround`)
          (set `self.Ele1st` false)
          (set `self.Ele2nd` false)
          (set `self.Ele3rdWin` false)
          (goto _label_5 :!via `Reverse`)))
      (elif (`self.Ele1st`)
        (if (`self.PlayerGround`)
          (set `self.Ele1st` false)
          (set `self.Ele2nd` false)
          (set `self.Ele3rdWin` false)
          (goto _label_6 :!via `Reverse`))
        (else
          (set `self.Ele1st` false)
          (set `self.Ele2nd` false)
          (set `self.Ele3rdWin` false))))))

(event `self.level1.OnComponentBeginOverlap`
  (params (OverlappedComponent :type "PrimitiveComponent Object Reference") (OtherActor :type "Actor Object Reference") (OtherComp :type "PrimitiveComponent Object Reference") (OtherBodyIndex :type Integer) (bFromSweep :type Boolean) (SweepResult :type "HitResult Structure (by ref)"))
  (set `self.PlayerGround` false)
  (set `self.Player1stfloor` true)
  (set `self.player2nd floor` false)
  (goto _label_7))

(event `self.Level2.OnComponentBeginOverlap`
  (params (OverlappedComponent :type "PrimitiveComponent Object Reference") (OtherActor :type "Actor Object Reference") (OtherComp :type "PrimitiveComponent Object Reference") (OtherBodyIndex :type Integer) (bFromSweep :type Boolean) (SweepResult :type "HitResult Structure (by ref)"))
  (set `self.PlayerGround` false)
  (set `self.Player1stfloor` false)
  (set `self.player2nd floor` true)
  (goto _label_7))

(fn `UserConstructionScript`)