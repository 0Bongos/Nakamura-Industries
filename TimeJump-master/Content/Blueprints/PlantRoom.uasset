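; PlantRoom drives a room where turning a wheel makes four plants rise or sink.
; Tick stores the Wheel's world pitch, then a five-second Delay gates the threshold check that plays or reverses a timeline.
; The timeline track, scaled by GrowHeight variables, sets each plant's relative Z from its own base offset while X and Y stay hard-coded.
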(event `self.ReceiveTick`
  (params (DeltaSeconds :type "Float (single-precision)"))
  (bind _grow_height_2 (`self.Grow height 2`))
  (bind _output_get (set `self.WheelRotation` (.pitch (`SceneComponent.K2_GetComponentRotation` (`self.Wheel`)))))
  (`KismetSystemLibrary.Delay` 5.0)
  (if (< _output_get -35.0)
    (bind (_direction _newtrack_0) (`Timeline|Timeline_0` :!label _label)
      (:`Update`
        (`self.K2_SetActorRelativeLocation` (`self.Plant 1`) (`KismetMathLibrary.MakeVector` -50.0 10490.0 (- (* _newtrack_0 (`self.Grow height 0`)) 890.0)) false false)
        (`self.K2_SetActorRelativeLocation` (`self.Plant 2`) (`KismetMathLibrary.MakeVector` -250.0 10280.0 (- (* _newtrack_0 _grow_height_2) 940.0)) false false)
        (`self.K2_SetActorRelativeLocation` (`self.Plant 3`) (`KismetMathLibrary.MakeVector` -460.0 10060.0 (- (* _newtrack_0 (`self.Grow height 1`)) 840.0)) false false)
        (`self.K2_SetActorRelativeLocation` (`self.Plant 4`) (`KismetMathLibrary.MakeVector` -680.0 9850.0 (- (* _newtrack_0 _grow_height_2) 880.0)) false false)))
    (else
      (goto _label :!via `Reverse`))))

(fn `UserConstructionScript`)