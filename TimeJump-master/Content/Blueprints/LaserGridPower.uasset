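; LaserGridPower is a trigger box that controls a laser gate and level 3 access on a referenced lift.
; When something enters the box, it revokes the lift's Level3Acess flag and shows the laser gate after a short delay.
; When the overlap ends, it grants access and flickers the gate on and off through a chain of delays before leaving it hidden.
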(event `self.Box.OnComponentBeginOverlap`
  (params (OverlappedComponent :type "PrimitiveComponent Object Reference") (OtherActor :type "Actor Object Reference") (OtherComp :type "PrimitiveComponent Object Reference") (OtherBodyIndex :type Integer) (bFromSweep :type Boolean) (SweepResult :type "HitResult Structure (by ref)"))
  (bind _aslift_blueprint (cast `/Game/Blueprints/Lift_blueprint` (`self.LiftReference`)))
  (set `/Game/Blueprints/Lift_blueprint.Level3Acess` false _aslift_blueprint)
  (`KismetSystemLibrary.Delay` 0.5)
  (`self.SetActorHiddenInGame` (`self.LaserGateReference`) false))

(event `self.Box.OnComponentEndOverlap`
  (params (OverlappedComponent :type "PrimitiveComponent Object Reference") (OtherActor :type "Actor Object Reference") (OtherComp :type "PrimitiveComponent Object Reference") (OtherBodyIndex :type Integer))
  (bind _lasergatereference (`self.LaserGateReference`))
  (bind _lasergatereference_2 (`self.LaserGateReference`))
  (bind _aslift_blueprint (cast `/Game/Blueprints/Lift_blueprint` (`self.LiftReference`)))
  (set `/Game/Blueprints/Lift_blueprint.Level3Acess` true _aslift_blueprint)
  (`KismetSystemLibrary.Delay` 0.5)
  (`self.SetActorHiddenInGame` _lasergatereference_2 true)
  (`KismetSystemLibrary.Delay` 0.5)
  (`self.SetActorHiddenInGame` _lasergatereference_2 false)
  (`KismetSystemLibrary.Delay` 0.5)
  (`self.SetActorHiddenInGame` _lasergatereference_2 true)
  (`KismetSystemLibrary.Delay` 0.5)
  (`self.SetActorHiddenInGame` _lasergatereference_2 false)
  (`KismetSystemLibrary.Delay` 0.5)
  (`self.SetActorHiddenInGame` _lasergatereference true)
  (`KismetSystemLibrary.Delay` 0.5)
  (`self.SetActorHiddenInGame` _lasergatereference false)
  (`KismetSystemLibrary.Delay` 0.5)
  (`self.SetActorHiddenInGame` _lasergatereference true))

(fn `UserConstructionScript`)