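; Locked double door that opens when a specific key actor, set by reference, enters its trigger box.
; A matching overlap turns its point light and a referenced DoorLight green, then plays a timeline.
; The timeline slides the referenced left and right door actors along X from hard-coded world positions, scaled by distance variables.
; The doors move only if the DoorLight cast succeeds, and nothing here closes them.
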(event `self.Box.OnComponentBeginOverlap`
  (params (OverlappedComponent :type "PrimitiveComponent Object Reference") (OtherActor :type "Actor Object Reference") (OtherComp :type "PrimitiveComponent Object Reference") (OtherBodyIndex :type Integer) (bFromSweep :type Boolean) (SweepResult :type "HitResult Structure (by ref)"))
  (set `self.CorrectKey` (== OtherActor (`self.KeyReference`)))
  (if (`self.CorrectKey`)
    (`LightComponent.SetLightColor` (`self.PointLight`) (struct :`R` 0.119792 :`G` 0.958333 :`B` 0.171363 :`A` 1.0) true)
    (bind _asdoor_light (cast `/Game/Blueprints/DoorLight` (`self.DoorLight`)))
    (`LightComponent.SetLightColor` (`Light.LightComponent` _asdoor_light) (struct :`R` 0.065592 :`G` 0.96875 :`B` 0.307653 :`A` 1.0) true)
    (bind (_direction _newtrack_0) (`Timeline|Timeline_1`)
      (:`Update`
        (`SceneComponent.K2_SetWorldLocation` (`Actor.RootComponent` (`self.DoorRight`)) (`KismetMathLibrary.MakeVector` (+ (* _newtrack_0 (`self.NegativeDistance`)) 2135.014648) 10009.987305 2552.5) false false)
        (`SceneComponent.K2_SetWorldLocation` (`Actor.RootComponent` (`self.DoorLeft`)) (`KismetMathLibrary.MakeVector` (+ (* _newtrack_0 (`self.OpenDistance`)) 2260.014648) 10009.986328 2552.5) false false)))))

(fn `UserConstructionScript`)