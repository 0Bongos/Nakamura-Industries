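; Box dropper actor that spawns companion cubes at a fixed world location, cycling through three colour variants.
; While StartPoop is true, Tick runs a five-second Delay that paces the spawns.
; Three booleans act as a rotating state, selecting default (white), green, then pink cube classes and handing off to the next colour after each spawn.
; StartPoop is only read here, never set.
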(event `self.ReceiveTick`
  (params (DeltaSeconds :type "Float (single-precision)"))
  (if (`self.StartPoop`)
    (`KismetSystemLibrary.Delay` 5.0)
    (if (`self.PoopWhite`)
      (`|SpawnActorFromClass` "/Game/Blueprints/CompanionCube.CompanionCube_C" (`KismetMathLibrary.MakeTransform` (4820.0 8680.0 3030.0)) "Undefined" "OverrideRootScale" null null)
      (set `self.PoopGreen` true)
      (set `self.PoopWhite` false)
      (set `self.PoopPink` false)
      (elif (`self.PoopGreen`)
        (`|SpawnActorFromClass` "/Game/Blueprints/CompanionCube_Green.CompanionCube_Green_C" (`KismetMathLibrary.MakeTransform` (4820.0 8680.0 3030.0)) "Undefined" "OverrideRootScale" null null)
        (set `self.PoopPink` true)
        (set `self.PoopGreen` false)
        (set `self.PoopWhite` false)
        (elif (`self.PoopPink`)
          (`|SpawnActorFromClass` "/Game/Blueprints/CompanionCube_Pink.CompanionCube_Pink_C" (`KismetMathLibrary.MakeTransform` (4820.0 8680.0 3030.0)) "Undefined" "OverrideRootScale" null null)
          (set `self.PoopWhite` true)
          (set `self.PoopPink` false)
          (set `self.PoopGreen` false))))))

(fn `UserConstructionScript`)