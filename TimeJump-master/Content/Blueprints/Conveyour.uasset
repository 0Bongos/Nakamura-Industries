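; Conveyor belt actor that carries objects along its forward direction and destroys colored cubes that reach its destroy volume.
; Every tick, components overlapping the Box are offset along the actor's forward vector by Speed and delta time, without sweeping.
; The Destory volume destroys overlapping pink, yellow or red cube actors and activates a particle effect.
; An unconnected older-style loop that moves only YellowCube actors never runs.
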(event `self.ReceiveTick`
  (params (DeltaSeconds :type "Float (single-precision)"))
  (for _array_element (`PrimitiveComponent.GetOverlappingComponents` (`self.Box`))
    (`SceneComponent.K2_AddWorldOffset` _array_element (* (`KismetMathLibrary.GetForwardVector` (`self.K2_GetActorRotation`)) (* DeltaSeconds (`self.Speed`))) false false)))

(event `self.Destory.OnComponentBeginOverlap`
  (params (OverlappedComponent :type "PrimitiveComponent Object Reference") (OtherActor :type "Actor Object Reference") (OtherComp :type "PrimitiveComponent Object Reference") (OtherBodyIndex :type Integer) (bFromSweep :type Boolean) (SweepResult :type "HitResult Structure (by ref)"))
  (if (or (== (`GameplayStatics.GetObjectClass` OtherActor) "/Game/Blueprints/PinkCube.PinkCube_C") (or (== "/Game/Blueprints/YellowCube.YellowCube_C" (`GameplayStatics.GetObjectClass` OtherActor)) (== "/Game/Blueprints/RedCube.RedCube_C" (`GameplayStatics.GetObjectClass` OtherActor))))
    (`self.K2_DestroyActor` OtherActor)
    (`ActorComponent.Activate` (`self.ParticleSystem`) false)))

(fn `UserConstructionScript`)