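; Final puzzle button that, when anything overlaps its trigger Box, clears a second volume and spawns a BlueCube.
; Overlap lights the mesh through the material's Active parameter and destroys all actors inside Box1.
; It then activates the particle system three times between short delays and spawns the cube at a hard-coded world location.
; Ending the overlap resets Active, with a new dynamic material instance created on each overlap event.
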(event `self.Box.OnComponentBeginOverlap`
  (params (OverlappedComponent :type "PrimitiveComponent Object Reference") (OtherActor :type "Actor Object Reference") (OtherComp :type "PrimitiveComponent Object Reference") (OtherBodyIndex :type Integer) (bFromSweep :type Boolean) (SweepResult :type "HitResult Structure (by ref)"))
  (bind _staticmeshcomponent (`self.StaticMeshComponent`))
  (bind _particlesystem (`self.ParticleSystem`))
  (`PrimitiveComponent.CreateDynamicMaterialInstance` _staticmeshcomponent 0 "/Game/Material/CubeMatss/CubeBase/Clean/CleanCubeBase-Mat_Inst.CleanCubeBase-Mat_Inst" "None")
  (`MeshComponent.SetScalarParameterValueOnMaterials` _staticmeshcomponent "Active" 120.0)
  (`self.K2_DestroyActor` (`PrimitiveComponent.GetOverlappingActors` (`self.Box1`) null))
  (`ActorComponent.Activate` _particlesystem false)
  (`KismetSystemLibrary.Delay` 0.2)
  (`ActorComponent.Activate` _particlesystem false)
  (`KismetSystemLibrary.Delay` 0.2)
  (`ActorComponent.Activate` _particlesystem false)
  (`KismetSystemLibrary.Delay` 0.5)
  (`|SpawnActorFromClass` "/Game/Blueprints/BlueCube.BlueCube_C" (`KismetMathLibrary.MakeTransform` (5831.0 7391.0 2883.0)) "Undefined" "OverrideRootScale" null null))

(event `self.Box.OnComponentEndOverlap`
  (params (OverlappedComponent :type "PrimitiveComponent Object Reference") (OtherActor :type "Actor Object Reference") (OtherComp :type "PrimitiveComponent Object Reference") (OtherBodyIndex :type Integer))
  (bind _staticmeshcomponent (`self.StaticMeshComponent`))
  (`PrimitiveComponent.CreateDynamicMaterialInstance` _staticmeshcomponent 0 "/Game/Material/CubeMatss/CubeBase/Clean/CleanCubeBase-Mat_Inst.CleanCubeBase-Mat_Inst" "None")
  (`MeshComponent.SetScalarParameterValueOnMaterials` _staticmeshcomponent "Active" 0.0))

(fn `UserConstructionScript`)