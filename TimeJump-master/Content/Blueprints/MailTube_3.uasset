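; Mail tube actor that carries actors along its length while powered, with a pressure-style trigger that switches it on.
; Overlapping Box1 turns the light green, powers the tube and plays a timeline moving a referenced Platform actor along Z; leaving reverses all three.
; While powered, Tick pushes everything overlapping the Capsule along the actor's forward vector at Speed.
; A separate Box trigger teleports entering actors to a hardcoded world location.
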(event `self.ReceiveTick`
  (params (DeltaSeconds :type "Float (single-precision)"))
  (if (`self.Powered`)
    (for _array_element (`PrimitiveComponent.GetOverlappingActors` (`self.Capsule`) null)
      (`self.K2_AddActorWorldOffset` _array_element (* (`KismetMathLibrary.GetForwardVector` (`self.K2_GetActorRotation`)) (* DeltaSeconds (`self.Speed`))) false false))))

(event `self.Box.OnComponentBeginOverlap`
  (params (OverlappedComponent :type "PrimitiveComponent Object Reference") (OtherActor :type "Actor Object Reference") (OtherComp :type "PrimitiveComponent Object Reference") (OtherBodyIndex :type Integer) (bFromSweep :type Boolean) (SweepResult :type "HitResult Structure (by ref)"))
  (`SceneComponent.K2_SetWorldLocation` (`Actor.RootComponent` OtherActor) (3689.955811 9133.543945 2865.0) false false))

(event `self.Box1.OnComponentBeginOverlap`
  (params (OverlappedComponent :type "PrimitiveComponent Object Reference") (OtherActor :type "Actor Object Reference") (OtherComp :type "PrimitiveComponent Object Reference") (OtherBodyIndex :type Integer) (bFromSweep :type Boolean) (SweepResult :type "HitResult Structure (by ref)"))
  (`LightComponent.SetLightColor` (`self.PointLight`) (struct :`R` 0.043735 :`G` 0.863157 :`B` 0.158961 :`A` 1.0) true)
  (set `self.Powered` true)
  (bind (_direction _newtrack_0) (`Timeline|Timeline_0` :!label _label)
    (:`Update`
      (`SceneComponent.K2_SetWorldLocation` (`Actor.RootComponent` (`self.Platform`)) (`KismetMathLibrary.MakeVector` 1640.0 11023.0 (+ (* _newtrack_0 (`self.AmoutTOMove`)) 2430.0)) false false))))

(event `self.Box1.OnComponentEndOverlap`
  (params (OverlappedComponent :type "PrimitiveComponent Object Reference") (OtherActor :type "Actor Object Reference") (OtherComp :type "PrimitiveComponent Object Reference") (OtherBodyIndex :type Integer))
  (`LightComponent.SetLightColor` (`self.PointLight`) (struct :`R` 0.863157 :`G` 0.017552 :`B` 0.043314 :`A` 1.0) true)
  (set `self.Powered` false)
  (goto _label :!via `Reverse`))

(fn `UserConstructionScript`)