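; PinkPower is a trigger-box switch that turns its point light green and moves a referenced platform while overlapped.
; A timeline scaled by Movement drives the platform along Y and Z from hard-coded world coordinates.
; Ending the overlap turns the light red and reverses the timeline.
; CorrectKey stores a comparison against CorrectCube, but the branch is fixed to true, so any overlap activates it.
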(event `self.Box.OnComponentBeginOverlap`
  (params (OverlappedComponent :type "PrimitiveComponent Object Reference") (OtherActor :type "Actor Object Reference") (OtherComp :type "PrimitiveComponent Object Reference") (OtherBodyIndex :type Integer) (bFromSweep :type Boolean) (SweepResult :type "HitResult Structure (by ref)"))
  (bind _movement (`self.Movement`))
  (set `self.CorrectKey` (== OverlappedComponent (`self.CorrectCube`)))
  (if true
    (`LightComponent.SetLightColor` (`self.PointLight`) (struct :`R` 0.119792 :`G` 0.958333 :`B` 0.171363 :`A` 1.0) true)
    (bind (_direction _newtrack_0) (`Timeline|Timeline_0` :!label _label)
      (:`Update`
        (`SceneComponent.K2_SetWorldLocation` (`Actor.RootComponent` (`self.PlatformRef`)) (`KismetMathLibrary.MakeVector` 5530.0 (+ (* _newtrack_0 _movement) 7650.0) (+ (* _newtrack_0 _movement) 2150.0)) false false)))))

(event `self.Box.OnComponentEndOverlap`
  (params (OverlappedComponent :type "PrimitiveComponent Object Reference") (OtherActor :type "Actor Object Reference") (OtherComp :type "PrimitiveComponent Object Reference") (OtherBodyIndex :type Integer))
  (`LightComponent.SetLightColor` (`self.PointLight`) (struct :`R` 0.958333 :`G` 0.007412 :`B` 0.0742 :`A` 1.0) true)
  (goto _label :!via `Reverse`))

(fn `UserConstructionScript`)