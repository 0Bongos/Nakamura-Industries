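; Cube base that powers on while something overlaps its Box and powers off when the overlap ends.
; Begin overlap plays on and looping-hum audio events and raises the material's "Active" parameter; end overlap stops the hum, plays the off event and zeroes it.
; A PowerOn flag guards the audio, while LazerGridOff limits a delayed laser-grid-off sound, triggered by end overlap, which only plays audio here.
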(event `self.Box.OnComponentBeginOverlap`
  (params (OverlappedComponent :type "PrimitiveComponent Object Reference") (OtherActor :type "Actor Object Reference") (OtherComp :type "PrimitiveComponent Object Reference") (OtherBodyIndex :type Integer) (bFromSweep :type Boolean) (SweepResult :type "HitResult Structure (by ref)"))
  (bind _staticmeshcomponent (`self.StaticMeshComponent`))
  (bind _box (`self.Box`))
  (if (not (`self.PowerOn`))
    (`FMODBlueprintStatics.PlayEventAtLocation` "/Game/FMOD/Events/Cube_Base_on.Cube_Base_on" (`KismetMathLibrary.Conv_VectorToTransform` (`SceneComponent.K2_GetComponentLocation` _box)))
    (bind _returnvalue (`FMODBlueprintStatics.PlayEventAtLocation` "/Game/FMOD/Events/Light_Hum_1.Light_Hum_1" (`KismetMathLibrary.Conv_VectorToTransform` (`SceneComponent.K2_GetComponentLocation` _box))))
    (set `self.PowerOn` true))
  (`PrimitiveComponent.CreateDynamicMaterialInstance` _staticmeshcomponent 0 "/Game/Material/CubeMatss/CubeBase/Clean/CleanCubeBase-Mat_Inst.CleanCubeBase-Mat_Inst" "None")
  (`MeshComponent.SetScalarParameterValueOnMaterials` _staticmeshcomponent "Active" 120.0))

(event `self.Box.OnComponentEndOverlap`
  (params (OverlappedComponent :type "PrimitiveComponent Object Reference") (OtherActor :type "Actor Object Reference") (OtherComp :type "PrimitiveComponent Object Reference") (OtherBodyIndex :type Integer))
  (bind _staticmeshcomponent (`self.StaticMeshComponent`))
  (bind _box (`self.Box`))
  (if (`self.PowerOn`)
    (`FMODBlueprintStatics.EventInstanceStop` (stale `self.Box.OnComponentBeginOverlap` _returnvalue))
    (`FMODBlueprintStatics.PlayEventAtLocation` "/Game/FMOD/Events/Cube_Base_off.Cube_Base_off" (`KismetMathLibrary.Conv_VectorToTransform` (`SceneComponent.K2_GetComponentLocation` _box)))
    (set `self.PowerOn` false))
  (`PrimitiveComponent.CreateDynamicMaterialInstance` _staticmeshcomponent 0 "/Game/Material/CubeMatss/CubeBase/Clean/CleanCubeBase-Mat_Inst.CleanCubeBase-Mat_Inst" "None")
  (`MeshComponent.SetScalarParameterValueOnMaterials` _staticmeshcomponent "Active" 0.0)
  (if (not (`self.LazerGridOff`))
    (`KismetSystemLibrary.Delay` 4.0)
    (`FMODBlueprintStatics.PlayEventAtLocation` "/Game/FMOD/Events/Lazer_grid_off.Lazer_grid_off" (`KismetMathLibrary.Conv_VectorToTransform` (`SceneComponent.K2_GetComponentLocation` _box)))
    (set `self.LazerGridOff` true)))

(fn `UserConstructionScript`)