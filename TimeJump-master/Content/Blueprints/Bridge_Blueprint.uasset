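; Bridge actor that tilts its static mesh according to the lever position of a referenced switch.
; Every Tick it sets the mesh's pitch from LeverPosition, keeping the actor's roll and yaw and feeding the mesh's world location back as its relative location.
; BeginPlay first sets the actor's relative location to that world location, then applies the same update.
; An unconnected check for the player holding the switch never runs.
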(event `self.ReceiveTick`
  (params (DeltaSeconds :type "Float (single-precision)"))
  (`SceneComponent.K2_SetRelativeLocationAndRotation` (`self.StaticMeshComponent`) (`SceneComponent.K2_GetComponentLocation` (`self.StaticMeshComponent`)) (`KismetMathLibrary.MakeRotator` (.roll (`self.K2_GetActorRotation`)) (* (`/Game/Blueprints/Switch.LeverPosition` (`self.SwitchReference`)) 1.0) (.yaw (`self.K2_GetActorRotation`))) false false :!label _label))

(event `self.ReceiveBeginPlay`
  (`self.K2_SetActorRelativeLocation` (`SceneComponent.K2_GetComponentLocation` (`self.StaticMeshComponent`)))
  (goto _label))

(fn `UserConstructionScript`)