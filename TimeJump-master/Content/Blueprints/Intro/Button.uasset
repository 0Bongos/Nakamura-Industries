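; Intro button Blueprint that slides a referenced bridge along X while its trigger box is overlapped.
; Begin overlap plays a timeline that scales TravelDistance from a fixed X offset, while end overlap reverses it from the end.
; The cast checks the Cube variable instead of the overlapping actor, so it does not filter what triggers the button.
; An equivalent SecondBridge move is present but never runs.
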(event `self.Box.OnComponentBeginOverlap`
  (params (OverlappedComponent :type "PrimitiveComponent Object Reference") (OtherActor :type "Actor Object Reference") (OtherComp :type "PrimitiveComponent Object Reference") (OtherBodyIndex :type Integer) (bFromSweep :type Boolean) (SweepResult :type "HitResult Structure (by ref)"))
  (bind (_returnvalue_x _returnvalue_y _returnvalue_z) (`KismetMathLibrary.BreakVector` (`SceneComponent.K2_GetComponentLocation` (`Actor.RootComponent` (`self.BridgeReference`)))))
  (cast `Actor` (`self.Cube`))
  (bind (_direction _newtrack_0) (`Timeline|Timeline_0` :!label _label)
    (:`Update`
      (`SceneComponent.K2_SetRelativeLocation` (`Actor.RootComponent` (`self.BridgeReference`)) (`KismetMathLibrary.MakeVector` (- (* _newtrack_0 (`self.TravelDistance`)) 1630.0) _returnvalue_y _returnvalue_z) false false))))

(event `self.Box.OnComponentEndOverlap`
  (params (OverlappedComponent :type "PrimitiveComponent Object Reference") (OtherActor :type "Actor Object Reference") (OtherComp :type "PrimitiveComponent Object Reference") (OtherBodyIndex :type Integer))
  (cast `Actor` (`self.Cube`))
  (goto _label :!via `ReverseFromEnd`))

(fn `UserConstructionScript`)