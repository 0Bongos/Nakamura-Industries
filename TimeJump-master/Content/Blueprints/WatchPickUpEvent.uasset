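; WatchPickUpEvent is a pickup actor that gives the first-person character a watch on overlap.
; The overlap sets the character's HasWatch flag, prints a debug string and plays a timeline.
; The timeline track, scaled by position and rotation variables, moves and yaws the Watch component from a fixed offset.
; A delay chained to the timeline's Update destroys the actor several seconds after the animation starts.
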(event `self.ReceiveActorBeginOverlap`
  (params (OtherActor :type "Actor Object Reference"))
  (bind _asfirst_person_character (cast `/Game/FirstPersonBP/Blueprints/FirstPersonCharacter` OtherActor))
  (set `/Game/FirstPersonBP/Blueprints/FirstPersonCharacter.HasWatch` true _asfirst_person_character)
  (`KismetSystemLibrary.PrintString` "Hello")
  (bind (_direction _newtrack_0) (`Timeline|Timeline_0`)
    (:`Update`
      (bind _returnvalue (* _newtrack_0 (`self.Position`)))
      (`SceneComponent.K2_SetRelativeLocationAndRotation` (`self.Watch`) (`KismetMathLibrary.MakeVector` 0.0 (- _returnvalue 60.0) (+ _returnvalue 51.0)) (`KismetMathLibrary.MakeRotator` 0.0 0.0 (* _newtrack_0 (`self.Rotaate`))) false false)
      (`KismetSystemLibrary.Delay` 8.0)
      (`self.K2_DestroyActor`))))

(fn `UserConstructionScript`)