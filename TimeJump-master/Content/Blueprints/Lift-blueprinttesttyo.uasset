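; Test lift Blueprint that moves the Lift component vertically when something begins overlapping its Box.
; The overlap plays a timeline whose track scales CurrentHeight plus one into the Lift's relative Z.
; CurrentHeight increments on every timeline update rather than once per trip.
; Floor-access checks and the fixed second and third step moves are unfinished, with nothing triggering them.
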(event `self.Box.OnComponentBeginOverlap`
  (params (OverlappedComponent :type "PrimitiveComponent Object Reference") (OtherActor :type "Actor Object Reference") (OtherComp :type "PrimitiveComponent Object Reference") (OtherBodyIndex :type Integer) (bFromSweep :type Boolean) (SweepResult :type "HitResult Structure (by ref)"))
  (bind (_direction _newtrack_0) (`Timeline|Timeline_0`)
    (:`Update`
      ;[1 1 1] +1
      (`SceneComponent.K2_SetRelativeLocation` (`self.Lift`) (`KismetMathLibrary.MakeVector` 0.0 0.0 (* _newtrack_0 (+ (`self.+1`) (`self.CurrentHeight`)))) false false)
      (set `self.CurrentHeight` (+ (`self.+1`) (`self.CurrentHeight`))))))

(fn `UserConstructionScript`)