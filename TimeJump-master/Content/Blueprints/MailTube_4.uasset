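; Mail tube puzzle actor that carries objects along its capsule while a base trigger powers it.
; Box1 overlap toggles power, base material, light color and FMOD audio, and plays or reverses a timeline moving a separate Platform vertically.
; While powered, Tick pushes capsule overlaps along actor forward, firing a whoosh per actor each frame.
; A second trigger, Box, teleports entering actors to a hard-coded world position, regardless of power.
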(event `self.ReceiveTick`
  (params (DeltaSeconds :type "Float (single-precision)"))
  (if (`self.Powered`)
    (for _array_element (`PrimitiveComponent.GetOverlappingActors` (`self.Capsule`) null)
      (`FMODBlueprintStatics.PlayEventAtLocation` "/Game/FMOD/Events/Mail_Tube_Whoosh.Mail_Tube_Whoosh" (`KismetMathLibrary.Conv_VectorToTransform` (`SceneComponent.K2_GetComponentLocation` (`self.Capsule`))))
      (`self.K2_AddActorWorldOffset` _array_element (* (`KismetMathLibrary.GetForwardVector` (`self.K2_GetActorRotation`)) (* DeltaSeconds (`self.Speed`))) false false))))

(event `self.Box.OnComponentBeginOverlap`
  (params (OverlappedComponent :type "PrimitiveComponent Object Reference") (OtherActor :type "Actor Object Reference") (OtherComp :type "PrimitiveComponent Object Reference") (OtherBodyIndex :type Integer) (bFromSweep :type Boolean) (SweepResult :type "HitResult Structure (by ref)"))
  (`SceneComponent.K2_SetWorldLocation` (`Actor.RootComponent` OtherActor) (3689.0 9133.0 2865.0) false false))

(event `self.Box1.OnComponentBeginOverlap`
  (params (OverlappedComponent :type "PrimitiveComponent Object Reference") (OtherActor :type "Actor Object Reference") (OtherComp :type "PrimitiveComponent Object Reference") (OtherBodyIndex :type Integer) (bFromSweep :type Boolean) (SweepResult :type "HitResult Structure (by ref)"))
  (bind _platform (`self.Platform`))
  (bind _rootcomponent (`Actor.RootComponent` _platform))
  (`FMODBlueprintStatics.PlayEventAtLocation` "/Game/FMOD/Events/Cube_Base_on.Cube_Base_on" (`KismetMathLibrary.Conv_VectorToTransform` (`SceneComponent.K2_GetComponentLocation` (`self.Base`))))
  (bind _returnvalue (`FMODBlueprintStatics.PlayEventAtLocation` "/Game/FMOD/Events/Light_Hum_1.Light_Hum_1" (`KismetMathLibrary.Conv_VectorToTransform` (`SceneComponent.K2_GetComponentLocation` (`self.Base`)))))
  (bind _returnvalue_2 (`FMODBlueprintStatics.PlayEventAtLocation` "/Game/FMOD/Events/Mail_Room_Buzz.Mail_Room_Buzz" (`KismetMathLibrary.Conv_VectorToTransform` (`SceneComponent.K2_GetComponentLocation` (`self.TubeFront`)))))
  (`PrimitiveComponent.CreateDynamicMaterialInstance` (`self.Base`) 0 "/Game/Material/CubeMatss/CubeBase/Clean/CleanCubeBase-Mat_Inst.CleanCubeBase-Mat_Inst" "None")
  (`MeshComponent.SetScalarParameterValueOnMaterials` (`self.Base`) "Active" 120.0)
  (`LightComponent.SetLightColor` (`self.PointLight`) (struct :`R` 0.043735 :`G` 0.863157 :`B` 0.158961 :`A` 1.0) true)
  (set `self.Powered` true)
  (bind (_direction _newtrack_0) (`Timeline|Timeline_0` :!label _label)
    (:`Update`
      (if (not (`self.MotionAudioOn`))
        (bind _returnvalue_3 (`FMODBlueprintStatics.PlayEventAtLocation` "/Game/FMOD/Events/Elevator_Motion.Elevator_Motion" (`KismetMathLibrary.Conv_VectorToTransform` (`SceneComponent.K2_GetComponentLocation` _rootcomponent))))
        (set `self.MotionAudioOn` true))
      (`SceneComponent.K2_SetWorldLocation` (`Actor.RootComponent` _platform) (`KismetMathLibrary.MakeVector` 1640.0 11023.0 (+ (* _newtrack_0 (`self.AmoutTOMove`)) 2430.0)) false false))
    (:`Finished`
      (`FMODBlueprintStatics.EventInstanceStop` _returnvalue_3)
      (`FMODBlueprintStatics.PlayEventAtLocation` "/Game/FMOD/Events/Elevator_stop.Elevator_stop" (`KismetMathLibrary.Conv_VectorToTransform` (`SceneComponent.K2_GetComponentLocation` _rootcomponent)))
      (set `self.MotionAudioOn` false))))

(event `self.Box1.OnComponentEndOverlap`
  (params (OverlappedComponent :type "PrimitiveComponent Object Reference") (OtherActor :type "Actor Object Reference") (OtherComp :type "PrimitiveComponent Object Reference") (OtherBodyIndex :type Integer))
  (`FMODBlueprintStatics.EventInstanceStop` (stale `self.Box1.OnComponentBeginOverlap` _returnvalue))
  (`FMODBlueprintStatics.EventInstanceStop` (stale `self.Box1.OnComponentBeginOverlap` _returnvalue_2))
  (`FMODBlueprintStatics.PlayEventAtLocation` "/Game/FMOD/Events/Cube_Base_off.Cube_Base_off" (`KismetMathLibrary.Conv_VectorToTransform` (`SceneComponent.K2_GetComponentLocation` (`self.Base`))))
  (`PrimitiveComponent.CreateDynamicMaterialInstance` (`self.Base`) 0 "/Game/Material/CubeMatss/CubeBase/Clean/CleanCubeBase-Mat_Inst.CleanCubeBase-Mat_Inst" "None")
  (`MeshComponent.SetScalarParameterValueOnMaterials` (`self.Base`) "Active" 0.0)
  (`LightComponent.SetLightColor` (`self.PointLight`) (struct :`R` 0.863157 :`G` 0.017552 :`B` 0.043314 :`A` 1.0) true)
  (set `self.Powered` false)
  (goto _label :!via `Reverse`))

(fn `UserConstructionScript`)