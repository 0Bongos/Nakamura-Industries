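; Painting lever actor that switches on scene lighting when its Lever component reaches a trigger Box.
; The first overlap of the Box by any component plays an FMOD thunk at the lever and sets a one-shot flag.
; If that component is the Lever, the point light turns cyan, four referenced light actors' roots become visible, and two post-process volumes' blend weights drop to zero.
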(event `self.ReceiveTick`
  (params (DeltaSeconds :type "Float (single-precision)")))

(event `self.Box.OnComponentBeginOverlap`
  (params (OverlappedComponent :type "PrimitiveComponent Object Reference") (OtherActor :type "Actor Object Reference") (OtherComp :type "PrimitiveComponent Object Reference") (OtherBodyIndex :type Integer) (bFromSweep :type Boolean) (SweepResult :type "HitResult Structure (by ref)"))
  (bind _lever (`self.Lever`))
  (if (not (`self.Thunked`))
    (`FMODBlueprintStatics.PlayEventAtLocation` "/Game/FMOD/Events/Pipe_Wheel_Thunk.Pipe_Wheel_Thunk" (`KismetMathLibrary.Conv_VectorToTransform` (`SceneComponent.K2_GetComponentLocation` _lever)))
    (set `self.Thunked` true)
    (if (== OtherComp _lever)
      (`LightComponent.SetLightColor` (`self.PointLight`) (struct :`G` 0.958333 :`B` 0.93693 :`A` 1.0) true)
      (`SceneComponent.SetVisibility` (`Actor.RootComponent` (`self.Lights`)) true false)
      (`SceneComponent.SetVisibility` (`Actor.RootComponent` (`self.Lights2`)) true false)
      (`SceneComponent.SetVisibility` (`Actor.RootComponent` (`self.Lights3`)) true false)
      (`SceneComponent.SetVisibility` (`Actor.RootComponent` (`self.Lights4`)) true false)
      (bind _aspost_process_volume (cast `PostProcessVolume` (`self.PostVolume`)))
      (set `PostProcessVolume.BlendWeight` 0.0 _aspost_process_volume)
      (bind _aspost_process_volume_2 (cast `PostProcessVolume` (`self.Postvolume2`)))
      (set `PostProcessVolume.BlendWeight` 0.0 _aspost_process_volume_2))))

(fn `UserConstructionScript`)