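; Plant room puzzle Blueprint where a turned pipe wheel waters and grows four potted plants.
; Every Tick checks the wheel's pitch: below zero it starts water particles, dripping audio and a one-shot thunk, otherwise it stops the water.
; The same check plays or reverses a timeline that sets each plant's height relative to its pot.
; Boolean latches prevent FMOD sounds retriggering, and timeline completion stops and resets the growth sounds.
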(event `self.ReceiveTick`
  (params (DeltaSeconds :type "Float (single-precision)"))
  (bind _particlesystem (`self.ParticleSystem`))
  (bind _grow_height_2 (`self.Grow height 2`))
  (bind (_returnvalue_x _returnvalue_y) (`KismetMathLibrary.BreakVector` (`self.K2_GetActorLocation` (`self.Pot4`))))
  (bind (_returnvalue_x_2 _returnvalue_y_2) (`KismetMathLibrary.BreakVector` (`self.K2_GetActorLocation` (`self.Pot3`))))
  (bind (_returnvalue_x_3 _returnvalue_y_3) (`KismetMathLibrary.BreakVector` (`self.K2_GetActorLocation` (`self.Pot2`))))
  (bind (_returnvalue_x_4 _returnvalue_y_4) (`KismetMathLibrary.BreakVector` (`self.K2_GetActorLocation` (`self.Pot1`))))
  (bind _output_get (set `self.WheelRotation` (.pitch (`SceneComponent.K2_GetComponentRotation` (`self.Wheel`)))))
  (bind _returnvalue (< _output_get 0.0))
  (if _returnvalue
    (`ActorComponent.Activate` _particlesystem false)
    (if (not (`self.Dripping`))
      (bind _returnvalue_2 (`FMODBlueprintStatics.PlayEventAtLocation` "/Game/FMOD/Events/Dripping_water.Dripping_water" (`KismetMathLibrary.Conv_VectorToTransform` (`SceneComponent.K2_GetComponentLocation` _particlesystem))))
      (set `self.Dripping` true))
    (else
      (set `self.Thunked` false)
      (`ActorComponent.Deactivate` _particlesystem)
      (`FMODBlueprintStatics.EventInstanceStop` _returnvalue_2)
      (set `self.Dripping` false)))
  (if _returnvalue
    (if (`self.Thunked`)
      (bind (_direction _newtrack_0) (`Timeline|Timeline_0` :!label _label)
        (:`Update`
          (if (not (`self.Plant1Grown`))
            (bind _returnvalue_3 (`FMODBlueprintStatics.PlayEventAtLocation` "/Game/FMOD/Events/Plant_Growth.Plant_Growth" (`KismetMathLibrary.Conv_VectorToTransform` (`SceneComponent.K2_GetComponentLocation` (`Actor.RootComponent` (`self.Plant 1`))))))
            (set `self.Plant1Grown` true))
          (`self.K2_SetActorRelativeLocation` (`self.Plant 1`) (`KismetMathLibrary.MakeVector` (+ _returnvalue_x_4 (`self.plusX`)) (- _returnvalue_y_4 (`self.minusY`)) (- (* _newtrack_0 (`self.Grow height 0`)) 890.0)) false false)
          (if (not (`self.Plant2Grown`))
            (bind _returnvalue_4 (`FMODBlueprintStatics.PlayEventAtLocation` "/Game/FMOD/Events/Plant_Growth.Plant_Growth" (`KismetMathLibrary.Conv_VectorToTransform` (`SceneComponent.K2_GetComponentLocation` (`Actor.RootComponent` (`self.Plant 2`))))))
            (set `self.Plant2Grown` true))
          (`self.K2_SetActorRelativeLocation` (`self.Plant 2`) (`KismetMathLibrary.MakeVector` (+ _returnvalue_x_3 (`self.plusX`)) (- _returnvalue_y_3 (`self.minusY`)) (- (* _newtrack_0 _grow_height_2) 940.0)) false false)
          (if (not (`self.Plant3Grown`))
            (bind _returnvalue_5 (`FMODBlueprintStatics.PlayEventAtLocation` "/Game/FMOD/Events/Plant_Growth.Plant_Growth" (`KismetMathLibrary.Conv_VectorToTransform` (`SceneComponent.K2_GetComponentLocation` (`Actor.RootComponent` (`self.Plant 3`))))))
            (set `self.Plant3Grown` true))
          (`self.K2_SetActorRelativeLocation` (`self.Plant 3`) (`KismetMathLibrary.MakeVector` (+ _returnvalue_x_2 (`self.plusX`)) (- _returnvalue_y_2 (`self.minusY`)) (- (* _newtrack_0 (`self.Grow height 1`)) 840.0)) false false)
          (if (not (`self.Plant4Grown`))
            (bind _returnvalue_6 (`FMODBlueprintStatics.PlayEventAtLocation` "/Game/FMOD/Events/Plant_Growth.Plant_Growth" (`KismetMathLibrary.Conv_VectorToTransform` (`SceneComponent.K2_GetComponentLocation` (`Actor.RootComponent` (`self.Plant 4`))))))
            (set `self.Plant4Grown` true))
          (`self.K2_SetActorRelativeLocation` (`self.Plant 4`) (`KismetMathLibrary.MakeVector` (+ _returnvalue_x (`self.plusX`)) (- _returnvalue_y (`self.minusY`)) (- (* _newtrack_0 _grow_height_2) 880.0)) false false))
        (:`Finished`
          (set `self.Plant1Grown` false)
          (set `self.Plant2Grown` false)
          (set `self.Plant3Grown` false)
          (set `self.Plant4Grown` false)
          (`FMODBlueprintStatics.EventInstanceStop` _returnvalue_3)
          (`FMODBlueprintStatics.EventInstanceStop` _returnvalue_4)
          (`FMODBlueprintStatics.EventInstanceStop` _returnvalue_5)
          (`FMODBlueprintStatics.EventInstanceStop` _returnvalue_6)))
      (else
        (`FMODBlueprintStatics.PlayEventAtLocation` "/Game/FMOD/Events/Pipe_Wheel_Thunk.Pipe_Wheel_Thunk" (`KismetMathLibrary.Conv_VectorToTransform` (`SceneComponent.K2_GetComponentLocation` (`self.Wheel`))))
        (set `self.Thunked` true)
        (goto _label)))
    (else
      (goto _label :!via `Reverse`))))

(fn `UserConstructionScript`)