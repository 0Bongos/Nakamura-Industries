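; Puzzle wheel actor that drives particle effects, plant growth and grill rusting from the wheel's rotation.
; Each Tick, negative pitch activates two particle systems and, while something overlaps the Box, plays a timeline raising the Plant at the Pot's position.
; It also swaps the grills for a spawned rusted version at a hardcoded transform.
; Non-negative pitch stops the particles, reverses the timeline and respawns intact grills.
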(event `self.ReceiveTick`
  (params (DeltaSeconds :type "Float (single-precision)"))
  (bind _rusted (`self.Rusted`))
  (bind _firstdestroy (`self.FirstDestroy`))
  (bind (_returnvalue_x _returnvalue_y _returnvalue_z) (`KismetMathLibrary.BreakVector` (`self.K2_GetActorLocation` (`self.Pot`))))
  (bind _rootcomponent (`Actor.RootComponent` (`self.Particle System`)))
  (bind _output_get (set `self.WheelRotation` (.pitch (`SceneComponent.K2_GetComponentRotation` (`self.Wheel`)))))
  (if (< _output_get 0.0)
    (`ActorComponent.Activate` _rootcomponent false)
    (`ActorComponent.Activate` (`Actor.RootComponent` (`self.SecondParticle`)) false)
    (`|ExecutionSequence`
      (:`then_0`
        (if (`self.Inplace`)
          (bind (_direction _newtrack_0) (`Timeline|Timeline_0` :!label _label)
            (:`Update`
              (`self.K2_SetActorRelativeLocation` (`self.Plant`) (`KismetMathLibrary.MakeVector` _returnvalue_x _returnvalue_y (+ (* _newtrack_0 (`self.Growth`)) (- _returnvalue_z 250.0))) false false)))))
      (:`then_1`
        (if (not _rusted)
          (`/Engine/EditorBlueprintResources/StandardMacros.IsValid` _firstdestroy
            (:`Is Valid`
              (`self.K2_DestroyActor` _firstdestroy))
            (:`Is Not Valid`
              _))
          (`/Engine/EditorBlueprintResources/StandardMacros.IsValid` (stale _returnvalue_2)
            (:`Is Valid`
              (`self.K2_DestroyActor` (stale _returnvalue_2)))
            (:`Is Not Valid`
              _))
          (bind _returnvalue (`|SpawnActorFromClass` "/Game/RustedGRILZ.RustedGRILZ_C" (`KismetMathLibrary.MakeTransform` (4357.0 7988.0 -429.0) (struct :`Yaw` 90.0)) "Undefined" "OverrideRootScale" null null))
          (set `self.Rusted` true))))
    (else
      (`ActorComponent.Deactivate` _rootcomponent)
      (`ActorComponent.Deactivate` (`Actor.RootComponent` (`self.SecondParticle`)))
      (`|ExecutionSequence`
        (:`then_0`
          (goto _label :!via `Reverse`))
        (:`then_1`
          (if _rusted
            (`self.K2_DestroyActor` _returnvalue)
            (bind _returnvalue_2 (`|SpawnActorFromClass` "/Game/Grills_GOOD.Grills_GOOD_C" (`KismetMathLibrary.MakeTransform` (4357.0 7988.0 -429.0) (struct :`Yaw` 90.0)) "Undefined" "OverrideRootScale" null null))
            (set `self.Rusted` false)))))))

(event `self.Box.OnComponentBeginOverlap`
  (params (OverlappedComponent :type "PrimitiveComponent Object Reference") (OtherActor :type "Actor Object Reference") (OtherComp :type "PrimitiveComponent Object Reference") (OtherBodyIndex :type Integer) (bFromSweep :type Boolean) (SweepResult :type "HitResult Structure (by ref)"))
  (set `self.Inplace` true))

(event `self.Box.OnComponentEndOverlap`
  (params (OverlappedComponent :type "PrimitiveComponent Object Reference") (OtherActor :type "Actor Object Reference") (OtherComp :type "PrimitiveComponent Object Reference") (OtherBodyIndex :type Integer))
  (set `self.Inplace` false))

(fn `UserConstructionScript`)