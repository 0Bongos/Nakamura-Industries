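; YellowPower is a cube-room trigger that powers moving platforms when a YellowCube enters its box.
; On overlap it clears StartPoop on the referenced BoxPooper_3Colour, turns its light green and plays three timelines sliding three referenced platforms along one axis each from hard-coded world positions.
; End overlap sets StartPoop again, turns the light red and reverses the timelines, without checking which actor left.
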(event `self.Box.OnComponentBeginOverlap`
  (params (OverlappedComponent :type "PrimitiveComponent Object Reference") (OtherActor :type "Actor Object Reference") (OtherComp :type "PrimitiveComponent Object Reference") (OtherBodyIndex :type Integer) (bFromSweep :type Boolean) (SweepResult :type "HitResult Structure (by ref)"))
  (bind _output_get (set `self.CorrectKey` (== "/Game/Blueprints/YellowCube.YellowCube_C" (`GameplayStatics.GetObjectClass` OtherActor))))
  (if _output_get
    (bind _asbox_pooper_3colour (cast `/Game/Blueprints/CubeRoom/BoxPooper_3Colour` (`self.BoxPooper`))
      (:`then`
        _)
      (:`CastFailed`
        _))
    (set `/Game/Blueprints/CubeRoom/BoxPooper_3Colour.StartPoop` false _asbox_pooper_3colour)
    (`|ExecutionSequence`
      (:`then_0`
        (`LightComponent.SetLightColor` (`self.PointLight`) (struct :`R` 0.119792 :`G` 0.958333 :`B` 0.171363 :`A` 1.0) true)
        (bind (_direction _newtrack_0) (`Timeline|Timeline_0` :!label _label)
          (:`Update`
            (`SceneComponent.K2_SetWorldLocation` (`Actor.RootComponent` (`self.PlatformRef`)) (`KismetMathLibrary.MakeVector` 4344.0 (+ (* _newtrack_0 (`self.Movement`)) 7974.0) 2065.0) false false))))
      (:`then_1`
        (bind (_direction_2 _newtrack_0_2) (`Timeline|Timeline_1` :!label _label_2)
          (:`Update`
            (`SceneComponent.K2_SetWorldLocation` (`Actor.RootComponent` (`self.PlatformRef2`)) (`KismetMathLibrary.MakeVector` (+ (* _newtrack_0_2 (`self.Movement2`)) 5845.0) 7387.0 2065.0) false false))))
      (:`then_2`
        (bind (_direction_3 _newtrack_0_3) (`Timeline|Timeline_2` :!label _label_3)
          (:`Update`
            (`SceneComponent.K2_SetWorldLocation` (`Actor.RootComponent` (`self.InactivePlat`)) (`KismetMathLibrary.MakeVector` 4344.0 (+ (* _newtrack_0_3 (`self.Movement`)) 7974.0) -785.0) false false)))))))

(event `self.Box.OnComponentEndOverlap`
  (params (OverlappedComponent :type "PrimitiveComponent Object Reference") (OtherActor :type "Actor Object Reference") (OtherComp :type "PrimitiveComponent Object Reference") (OtherBodyIndex :type Integer))
  (bind _asbox_pooper_3colour (cast `/Game/Blueprints/CubeRoom/BoxPooper_3Colour` (`self.BoxPooper`)))
  (set `/Game/Blueprints/CubeRoom/BoxPooper_3Colour.StartPoop` true _asbox_pooper_3colour)
  (`LightComponent.SetLightColor` (`self.PointLight`) (struct :`R` 0.958333 :`G` 0.007412 :`B` 0.0742 :`A` 1.0) true)
  (`|ExecutionSequence`
    (:`then_0`
      (goto _label :!via `Reverse`))
    (:`then_1`
      (goto _label_2 :!via `Reverse`))
    (:`then_2`
      (goto _label_3 :!via `Reverse`))))

(fn `UserConstructionScript`)