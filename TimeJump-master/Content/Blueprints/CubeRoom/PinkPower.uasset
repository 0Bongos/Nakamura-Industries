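; PinkPower is a cube-activated trigger in the CubeRoom that opens a pair of moving pieces and raises steps.
; A BlueCube entering the Box turns the PointLight green and plays timelines that slide Left and Right along Y and lift and pitch the steps.
; Any end overlap, without a class check, turns the light red and reverses the timelines.
; Target positions are hardcoded world coordinates, offset by timeline-scaled variables.
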(event `self.Box.OnComponentBeginOverlap`
  (params (OverlappedComponent :type "PrimitiveComponent Object Reference") (OtherActor :type "Actor Object Reference") (OtherComp :type "PrimitiveComponent Object Reference") (OtherBodyIndex :type Integer) (bFromSweep :type Boolean) (SweepResult :type "HitResult Structure (by ref)"))
  (bind _output_get (set `self.CorrectKey` (== "/Game/Blueprints/BlueCube.BlueCube_C" (`GameplayStatics.GetObjectClass` OtherActor))))
  (if _output_get
    (`LightComponent.SetLightColor` (`self.PointLight`) (struct :`R` 0.119792 :`G` 0.958333 :`B` 0.171363 :`A` 1.0) true)
    (`|ExecutionSequence`
      (:`then_0`
        (bind (_direction _newtrack_0) (`Timeline|Timeline_0` :!label _label)
          (:`Update`
            (`SceneComponent.K2_SetWorldLocation` (`Actor.RootComponent` (`self.Left`)) (`KismetMathLibrary.MakeVector` 5827.0 (+ (* _newtrack_0 (`self.Movement`)) 7294.0) 2408.0) false false))))
      (:`then_1`
        (bind (_direction_2 _newtrack_0_2) (`Timeline|Timeline_1` :!label _label_2)
          (:`Update`
            (`SceneComponent.K2_SetWorldLocation` (`Actor.RootComponent` (`self.Right`)) (`KismetMathLibrary.MakeVector` 5827.0 (+ (* _newtrack_0_2 (`self.Movement+`)) 7494.0) 2408.0) false false))))
      (:`then_2`
        (bind (_direction_3 _newtrack_0_3) (`Timeline|Timeline_2` :!label _label_3)
          (:`Update`
            (`self.K2_SetActorLocationAndRotation` (`self.Step1`) (`KismetMathLibrary.MakeVector` 4431.0 7533.0 (+ (* _newtrack_0_3 (`self.Srep`)) 2410.0)) (`KismetMathLibrary.MakeRotator` 0.0 (* _newtrack_0_3 -18.0)) false false))))
      (:`then_3`
        (bind (_direction_4 _newtrack_0_4) (`Timeline|Timeline_3` :!label _label_4)
          (:`Update`
            (`self.K2_SetActorLocationAndRotation` (`self.Step 2`) (`KismetMathLibrary.MakeVector` 4589.0 7533.0 (+ (* _newtrack_0_4 (* (`self.Srep`) 2.0)) 2410.0)) (`KismetMathLibrary.MakeRotator` 0.0 (* _newtrack_0_4 -18.0)) false false))))
      (:`then_4`
        (bind (_direction_5 _newtrack_0_5) (`Timeline|Timeline_4` :!label _label_5)
          (:`Update`
            (`self.K2_SetActorLocationAndRotation` (`self.Step 3`) (`KismetMathLibrary.MakeVector` 4747.0 7533.0 (+ (* _newtrack_0_5 (* (`self.Srep`) 3.0)) 2410.0)) (`KismetMathLibrary.MakeRotator` 0.0 (* _newtrack_0_5 -18.0)) false false))))
      (:`then_5`
        (bind (_direction_6 _newtrack_0_6) (`Timeline|Timeline_5` :!label _label_6)
          (:`Update`
            (`self.K2_SetActorRotation` (`self.Step0`) (`KismetMathLibrary.MakeRotator` 0.0 (* _newtrack_0_6 -18.0)) false)))))))

(event `self.Box.OnComponentEndOverlap`
  (params (OverlappedComponent :type "PrimitiveComponent Object Reference") (OtherActor :type "Actor Object Reference") (OtherComp :type "PrimitiveComponent Object Reference") (OtherBodyIndex :type Integer))
  (`LightComponent.SetLightColor` (`self.PointLight`) (struct :`R` 0.958333 :`G` 0.007412 :`B` 0.0742 :`A` 1.0) true)
  (`|ExecutionSequence`
    (:`then_0`
      (goto _label :!via `Reverse`))
    (:`then_1`
      (goto _label_2 :!via `Reverse`))
    (:`then_2`
      (goto _label_3 :!via `Reverse`))
    (:`then_3`
      (goto _label_4 :!via `Reverse`))
    (:`then_4`
      (goto _label_5 :!via `Reverse`))
    (:`then_5`
      (goto _label_6 :!via `Reverse`))))

(fn `UserConstructionScript`)