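; ButtonLevel1_2 is a trigger button that slides two door actors open while something overlaps its box and closes them when the overlap ends.
; A timeline plays forward on begin overlap and reverses on end overlap.
; Its track scales separate distance variables to offset each door along world X from hardcoded closed positions.
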(event `self.Box.OnComponentBeginOverlap`
  (params (OverlappedComponent :type "PrimitiveComponent Object Reference") (OtherActor :type "Actor Object Reference") (OtherComp :type "PrimitiveComponent Object Reference") (OtherBodyIndex :type Integer) (bFromSweep :type Boolean) (SweepResult :type "HitResult Structure (by ref)"))
  (bind (_direction _newtrack_0) (`Timeline|Timeline_0` :!label _label)
    (:`Update`
      (`SceneComponent.K2_SetWorldLocation` (`Actor.RootComponent` (`self.DoorLeft`)) (`KismetMathLibrary.MakeVector` (+ (* _newtrack_0 (`self.NegativeDistance`)) 2050.001465) 6429.625977 2186.0) false false)
      (`SceneComponent.K2_SetWorldLocation` (`Actor.RootComponent` (`self.DoorRight`)) (`KismetMathLibrary.MakeVector` (+ (* _newtrack_0 (`self.OpenDistance`)) 3720.216064) 6942.983398 2186.0) false false))))

(event `self.Box.OnComponentEndOverlap`
  (params (OverlappedComponent :type "PrimitiveComponent Object Reference") (OtherActor :type "Actor Object Reference") (OtherComp :type "PrimitiveComponent Object Reference") (OtherBodyIndex :type Integer))
  (goto _label :!via `Reverse`))

(fn `UserConstructionScript`)